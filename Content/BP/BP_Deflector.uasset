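; BP_Deflector is an actor that the player rotates by holding the 1 key.
; The key opens and closes a Gate on Tick, which adds a fixed, frame-rate-dependent yaw step each frame.
; Tick also polls the Lerp scalar in the LerpMPC parameter collection and disables input when it equals 1.
; A GreenLight material swap on the same condition is unconnected and never runs.
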(event EventBeginPlay
  (Input|EnableInput (Game|GetPlayerController 0)))

(event Collision|EventActorBeginOverlap
  (params (OtherActor :type Actor%20Object%20Reference)))

(event EventTick
  (params (DeltaSeconds :type Float%20%28single-precision%29))
  (Utilities|FlowControl|Sequence
    (:then_0
      (bind _output_get (Variables|Default|SetCurrentZ (.yaw (Transformation|GetActorRotation))))
      (Utilities|FlowControl|Gate true
        (:Exit
          (bind _output_get_2 (Variables|Default|SetCurrentZ (+ _output_get 0.2)))
          (Transformation|SetActorRotation (Math|Rotator|MakeRotator 0.0 0.0 _output_get_2)))))
    (:then_1
      (bind _returnvalue (Rendering|Material|GetScalarParameterValue "/Game/Materials/LerpMPC.LerpMPC" "Lerp" :!class /Script/Engine.KismetMaterialLibrary))
      (if (== _returnvalue 1.0)
        (Input|DisableInput (Game|GetPlayerController 0))))))

(event Input|KeyboardEvents|1
  (params (Key :type Key%20Structure :default "None"))
  (:Pressed
    (Utilities|FlowControl|Gate true) ; enters at Open
  )
  (:Released
    (Utilities|FlowControl|Gate true) ; enters at Close
  ))

(fn ConstructionScript)